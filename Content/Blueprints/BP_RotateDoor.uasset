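; BP_RotateDoor is a hinged door that the player opens once with the Interact action.
; TriggerBox overlap enables input on the door and sets the player's interact prompt, and leaving reverses both.
; Interact snaps the Hinge to a fixed rotation without animation, then destroys TriggerBox so the door has no way to close.
; Guard enemy overlaps are cast-checked but trigger no action.
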(event `self.TriggerBox.OnComponentBeginOverlap`
  (params (OverlappedComponent :type "PrimitiveComponent Object Reference") (OtherActor :type "Actor Object Reference") (OtherComp :type "PrimitiveComponent Object Reference") (OtherBodyIndex :type Integer) (bFromSweep :type Boolean) (SweepResult :type "HitResult Structure (by ref)"))
  ; Taken from BP_Door
  (bind _asbp_player (cast `/Game/Blueprints/BP_Player` OtherActor)
    (:`then`
      (`self.EnableInput` (`GameplayStatics.GetPlayerController` 0))
      (set `/Game/Blueprints/BP_Player.CurrentInteractText` "E - Open Door" _asbp_player))
    (:`CastFailed`
      (cast `/Game/Blueprints/GuardCharacter/BP_GuardEnemy` OtherActor))))

(event `InputAction|Interact`
  (params (Key :type "Key Structure"))
  ; Taken from BP_Door
  (:`Pressed`
    (`SceneComponent.K2_SetRelativeRotation` (`self.Hinge`) (struct :`Yaw` 90.0) false false)
    (`ActorComponent.K2_DestroyComponent` (`self.TriggerBox`))))

(event `self.TriggerBox.OnComponentEndOverlap`
  (params (OverlappedComponent :type "PrimitiveComponent Object Reference") (OtherActor :type "Actor Object Reference") (OtherComp :type "PrimitiveComponent Object Reference") (OtherBodyIndex :type Integer))
  ; Taken from BP_Door
  (bind _asbp_player (cast `/Game/Blueprints/BP_Player` OtherActor)
    (:`then`
      (`self.DisableInput` (`GameplayStatics.GetPlayerController` 0))
      (set `/Game/Blueprints/BP_Player.CurrentInteractText` "" _asbp_player))
    (:`CastFailed`
      (cast `/Game/Blueprints/GuardCharacter/BP_GuardEnemy` OtherActor))))

(fn `UserConstructionScript`)