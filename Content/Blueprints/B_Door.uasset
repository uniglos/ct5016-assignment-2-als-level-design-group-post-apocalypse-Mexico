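; Door actor that opens when enough linked pressure switches are active.
; SwitchActivated and SwitchDeactivated events raise or lower an active-switch count and compare it to the required number.
; Meeting the threshold plays a timeline that moves the door mesh along relative Z, and falling short reverses it.
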(event `SwitchActivated`
  (`/Engine/EditorBlueprintResources/StandardMacros.IncrementInt` (`self.PressureSwitchesActive`)
    (:`  `
      (if (>= (`self.PressureSwitchesActive`) (`self.PressureSwitchesNeeded`))
        (bind (_direction _doorposition) (`Timeline|Doormovement` :!label _label)
          (:`Update`
            (`SceneComponent.K2_SetRelativeLocation` (`self.Door`) (`KismetMathLibrary.MakeVector` 0.0 0.0 _doorposition) false false)))
        (else
          (goto _label :!via `Reverse`))))))

(event `SwitchDeactivated`
  (`/Engine/EditorBlueprintResources/StandardMacros.DecrementInt` (`self.PressureSwitchesActive`)
    (:`  `
      (if (>= (`self.PressureSwitchesActive`) (`self.PressureSwitchesNeeded`))
        (goto _label)
        (else
          (goto _label :!via `Reverse`))))))

(fn `UserConstructionScript`)